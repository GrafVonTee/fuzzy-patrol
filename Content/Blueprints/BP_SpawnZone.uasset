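; Spawn zone actor that lets the player place enemies inside it with mouse clicks.
; It enables input on BeginPlay, then left click spawns a visible enemy and right click an invisible one.
; SpawnEnemy traces from the cursor into the world and proceeds only if it hits a spawn zone.
; Enemies spawn at the hit X and Y and the hit component's Z, adjusted for collisions or skipped.
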(event EventBeginPlay
  (bind _output_get (Variables|Default|SetController (Game|GetPlayerController 0)))
  (Input|EnableInput _output_get))

(event Collision|EventActorBeginOverlap
  (params (OtherActor :type Actor%20Object%20Reference)))

(event EventTick
  (params (DeltaSeconds :type Float%20%28single-precision%29)))

(event Input|MouseEvents|LeftMouseButton
  (params (Key :type Key%20Structure :default "None"))
  (:Pressed
    (CallFunction|SpawnEnemy "/Game/Blueprints/Enemies/BP_VisibleEnemy.BP_VisibleEnemy_C")))

(event Input|MouseEvents|RightMouseButton
  (params (Key :type Key%20Structure :default "None"))
  (:Pressed
    (CallFunction|SpawnEnemy "/Game/Blueprints/Enemies/BP_InvisibleEnemy.BP_InvisibleEnemy_C")))

(fn ConstructionScript)

(fn SpawnEnemy
  (params (EnemyClass :type Default%20Enemy%20Class%20Reference))
  (bind _controller (Variables|Default|GetController))
  (bind (_worldlocation _worlddirection) (Game|Player|ConvertMouseLocationToWorldSpace _controller))
  (bind (_outhit _returnvalue) (Collision|LineTraceForObjects _worldlocation (+ _worldlocation (* _worlddirection 1e+04)) (Variables|Default|GetObject%20Types) false 0 "None" false))
  (if _returnvalue
    (Utilities|Casting|CastToBP_SpawnZone (.HitActor (Collision|BreakHitResult _outhit)))
    (Game|SpawnActorfromClass EnemyClass (Math|Transform|MakeTransform (Math|Vector|MakeVector (.X (Math|Vector|BreakVector (.Location (Collision|BreakHitResult _outhit)))) (.Y (Math|Vector|BreakVector (.Location (Collision|BreakHitResult _outhit)))) (.z (Transformation|GetWorldLocation (.HitComponent (Collision|BreakHitResult _outhit))))) "0, 0, 0" "1,1,1") "AdjustIfPossibleButDontSpawnIfColliding" 0 0)))