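; BP_TeaReceiver is an environment zone that lets overlapping BP_PatrolAgent actors receive tea.
; On begin overlap it enables the agent's ReceivingComponent with its QuenchPeriod and TeaValue, retrying every half second while that component is invalid.
; On end overlap it disables receiving, without a validity check.
; The construction script sets the Cylinder's world scale to its relative scale.
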(event EventBeginPlay)

(event EventTick
  (params (DeltaSeconds :type Float%20%28single-precision%29)))

(event Collision|EventActorBeginOverlap
  (params (OtherActor :type Actor%20Object%20Reference))
  (bind _asbp_patrol_agent (Utilities|Casting|CastToBP_PatrolAgent OtherActor :!label _label))
  (if (Utilities|IsValid (Variables|/Script/FuzzyPatrol.PatrolAgent|GetReceivingComponent _asbp_patrol_agent))
    (Class|ReceivingComponent|EnableReceiving (Variables|/Script/FuzzyPatrol.PatrolAgent|GetReceivingComponent _asbp_patrol_agent) (Variables|Default|GetQuenchPeriod) (Variables|Default|GetTeaValue))
    (else
      (Utilities|FlowControl|Delay 0.5)
      (goto _label))))

(event Collision|EventActorEndOverlap
  (params (OtherActor :type Actor%20Object%20Reference))
  (bind _asbp_patrol_agent (Utilities|Casting|CastToBP_PatrolAgent OtherActor))
  (Class|ReceivingComponent|DisableReceiving (Variables|/Script/FuzzyPatrol.PatrolAgent|GetReceivingComponent _asbp_patrol_agent)))

(fn ConstructionScript
  (bind _cylinder (Variables|Default|GetCylinder))
  (Transformation|SetWorldScale3D _cylinder (Variables|/Script/Engine.SceneComponent|GetRelativeScale3D _cylinder)))