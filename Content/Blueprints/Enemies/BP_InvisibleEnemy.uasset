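; BP_InvisibleEnemy is a temporary enemy actor that replaces itself with a BP_VisibleEnemy after a set lifetime.
; BeginPlay starts a one-shot timer using LifePeriod, bound to the DestroyItself event.
; When it fires, DestroyItself always spawns the visible enemy at the actor's current location, regardless of collision, then destroys this actor.
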(event Custom|Destroy%20Itself
  (Game|SpawnActorfromClass "/Game/Blueprints/Enemies/BP_VisibleEnemy.BP_VisibleEnemy_C" (Math|Transform|MakeTransform (Transformation|GetActorLocation) "0, 0, 0" "1,1,1") "AlwaysSpawn" 0 0)
  (Actor|DestroyActor))

(event EventBeginPlay
  (|CallParentFunction)
  (Utilities|Time|SetTimerbyEvent (delegate Custom|Destroy%20Itself) (Variables|Default|GetLife%20Period)))

(event Collision|EventActorBeginOverlap
  (params (OtherActor :type Actor%20Object%20Reference))
  (|CallParentFunction OtherActor) ; This node is disabled and will not be called.\nDrag off pins to build functionality.
)

(event EventTick
  (params (DeltaSeconds :type Float%20%28single-precision%29))
  (|CallParentFunction DeltaSeconds) ; This node is disabled and will not be called.\nDrag off pins to build functionality.
)

(fn ConstructionScript
  (|CallParentFunction))