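; Default enemy that wanders to random points and flashes when damaged, with its body built from top and bottom cone components.
; MoveToRandom sends it via AI MoveTo to a random reachable point within PathFindRadius, retrying only when the move fails.
; PlayAnimationReceivingDamage briefly swaps both cones to a damaged material, then applies the top cone's cached material to both.
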(event EventBeginPlay)

(event Collision|EventActorBeginOverlap
  (params (OtherActor :type Actor%20Object%20Reference)))

(event EventTick
  (params (DeltaSeconds :type Float%20%28single-precision%29)))

(event EventMovetoRandom
  (AI|AIMoveTo self (.RandomLocation (AI|Navigation|GetRandomReachablePointinRadius (Transformation|GetActorLocation) (Variables|Default|GetPathFindRadius) 0 0)) 0 5.0 false
    (:OnFail
      (Class|DefaultEnemy|MovetoRandom))))

(event EventPlayAnimationReceivingDamage
  (Variables|Default|SetOriginal%20Material (Rendering|Material|GetMaterial (Variables|Default|GetTopCone) 0))
  (Rendering|Material|SetMaterial (Variables|Default|GetTopCone) 0 "/Game/Materials/M_DamagedEnemy.M_DamagedEnemy")
  (Utilities|FlowControl|Delay 0.3)
  (Rendering|Material|SetMaterial (Variables|Default|GetTopCone) 0 (Variables|Default|GetOriginal%20Material)))

(fn ConstructionScript)